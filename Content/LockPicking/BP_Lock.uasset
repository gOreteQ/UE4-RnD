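; BP_Lock is an interactable lock that runs a lockpicking minigame through a W_Lock widget.
; It picks a random sweet-spot angle, with tolerances from a difficulty data table.
; RotatePin and RotateLock drive the widget angles, and a cosine falloff caps lock rotation by pin accuracy.
; Forcing a misaligned pin wiggles it and wears down the character's picks, while reaching 90 degrees unlocks and restores input.
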(event Custom|Wiggle
  (Variables|Default|SetPinRotation (Math|Float|Clamp(Float) (Math|Random|RandomFloatinRange (- (Variables|Default|GetPinRotation) 1.0) (+ (Variables|Default|GetPinRotation) 1.0)) -9e+01 9e+01))
  (Variables|Default|SetLockRotation (Math|Float|Clamp(Float) (Math|Random|RandomFloatinRange (- (Variables|Default|GetLockRotation) 1.0) (+ (Variables|Default|GetLockRotation) 1.0)) 0.0 9e+01)))

(event Custom|RotateLock
  (params (Rotation :type Float%20%28single-precision%29))
  (bind _pinrotation (Variables|Default|GetPinRotation))
  (if (and (== Rotation 0.0) (> (Variables|Default|GetLockRotation) 1.0))
    (Variables|Default|SetLockRotation (- (Variables|Default|GetLockRotation) (* 45.0 (Variables|Default|GetDeltaTime))))
    (elif (> (Variables|/Game/Player/BP_RnDChar.BP_RnDChar_C|GetPickAmount (.AsBP%20Rn%20DChar (Utilities|Casting|CastToBP_RnDChar (Variables|Default|GetCaller)))) 0)
      (if (== Rotation 1.0)
        (if (and (> _pinrotation (- (Variables|Default|GetUnlockRotation) (Variables|Default|GetRotateTolerance))) (< _pinrotation (+ (Variables|Default|GetUnlockRotation) (Variables|Default|GetRotateTolerance))))
          (Variables|Default|SetbCanRotate true)
          (if (Math|Float|InRange(Float) (Variables|Default|GetPinRotation) (- (Variables|Default|GetUnlockRotation) (Variables|Default|GetUnlockTolerance)) (+ (Variables|Default|GetUnlockRotation) (Variables|Default|GetUnlockTolerance)))
            (Variables|Default|SetLockMaxRot 9e+01)
            (else
              (Variables|Default|SetLockMaxRot (* (|(cosd(((abs((unlock-pin)))*coeff))) (Variables|Default|GetUnlockRotation) (Variables|Default|GetPinRotation) (/ 8e+01 (Variables|Default|GetRotateTolerance))) 9e+01))))
          (Variables|Default|SetLockRotation (Math|Float|Clamp(Float) (+ (Variables|Default|GetLockRotation) (* Rotation 45.0 (Variables|Default|GetDeltaTime))) 0.0 (Variables|Default|GetLockMaxRot)))
          (if (and (== (Variables|Default|GetLockRotation) (Variables|Default|GetLockMaxRot)) (!= (Variables|Default|GetLockMaxRot) 9e+01))
            (CallFunction|DamagePick))
          (else
            (Variables|Default|SetbCanRotate false)
            (CallFunction|DamagePick))))
      (else
        (Development|PrintString "Oh no! You have no picks left!!")))))

(event Custom|RotatePin
  (params (Rotation :type Float%20%28single-precision%29))
  (if (< (Variables|Default|GetLockRotation) 1.0)
    (Variables|Default|SetPinRotation (Math|Float|Clamp(Float) (+ Rotation (Variables|Default|GetPinRotation)) -9e+01 9e+01))))

(event Custom|Unlock
  (Variables|Default|SetbIsLocked false)
  (Variables|Default|SetbIsActive false)
  (Widget|RemovefromParent (Variables|Default|GetLockWidget))
  (Variables|/Game/Player/BP_RnDChar.BP_RnDChar_C|SetbAllowInput (.AsBP%20Rn%20DChar (Utilities|Casting|CastToBP_RnDChar (Variables|Default|GetCaller))) true))

(event Custom|DamagePick
  (bind _caller (Variables|Default|GetCaller))
  (bind _asbp_rn_dchar (Utilities|Casting|CastToBP_RnDChar _caller))
  (CallFunction|Wiggle)
  (bind _output_get (Variables|/Game/Player/BP_RnDChar.BP_RnDChar_C|SetPickHP _asbp_rn_dchar (- (Variables|/Game/Player/BP_RnDChar.BP_RnDChar_C|GetPickHP _asbp_rn_dchar) (* 5e+01 (Variables|Default|GetDeltaTime)))))
  (if (<= _output_get 0.0)
    (Development|PrintString (Utilities|String|Append "Oh no! Your pick broke! You have " (Utilities|String|ToString(Integer) (- (Variables|/Game/Player/BP_RnDChar.BP_RnDChar_C|GetPickAmount _asbp_rn_dchar) 1)) " picks left!"))
    (Variables|/Game/Player/BP_RnDChar.BP_RnDChar_C|SetPickHP _asbp_rn_dchar 1e+02)
    (Variables|/Game/Player/BP_RnDChar.BP_RnDChar_C|SetPickAmount _asbp_rn_dchar (- (Variables|/Game/Player/BP_RnDChar.BP_RnDChar_C|GetPickAmount _asbp_rn_dchar) 1))
    (Variables|Default|SetPinRotation 0.0)
    (Variables|Default|SetLockRotation 0.0)))

(event EventTick
  (params (DeltaSeconds :type Float%20%28single-precision%29))
  (bind _lockwidget (Variables|Default|GetLockWidget))
  (bind _pinrotation (Variables|Default|GetPinRotation))
  (Variables|Default|SetDeltaTime DeltaSeconds)
  (if (Variables|Default|GetbIsActive)
    (Class|Widget|SetRenderAngle (Variables|/Game/LockPicking/W_Lock.W_Lock_C|GetPin _lockwidget) _pinrotation)
    (Class|Widget|SetRenderAngle (Variables|/Game/LockPicking/W_Lock.W_Lock_C|GetLock _lockwidget) (Variables|Default|GetLockRotation))
    (Development|PrintString (Utilities|String|Append (Utilities|String|ToString(Float) _pinrotation) " | " (Utilities|String|ToString(Float) (Variables|Default|GetUnlockRotation)) " | " (Utilities|String|ToString(Boolean) (Variables|Default|GetbCanRotate)) " | " (Utilities|String|ToString(Float) (Variables|Default|GetLockRotation))) true true "(R=0.000000,G=0.660000,B=1.000000,A=1.000000)" 0.0)
    (if (== (Variables|Default|GetLockRotation) 9e+01)
      (CallFunction|Unlock))))

(event EventInteract
  (params (Caller :type Actor%20Object%20Reference))
  (bind _output_get (Variables|Default|SetCaller Caller))
  (Variables|/Game/Player/BP_RnDChar.BP_RnDChar_C|SetbAllowInput (.AsBP%20Rn%20DChar (Utilities|Casting|CastToBP_RnDChar _output_get)) false)
  (if (> (Variables|/Game/Player/BP_RnDChar.BP_RnDChar_C|GetPickAmount (.AsBP%20Rn%20DChar (Utilities|Casting|CastToBP_RnDChar _output_get))) 0)
    (if (Variables|Default|GetbIsLocked)
      (if (== (Variables|Default|GetLockWidget) 0)
        (bind _returnvalue (UserInterface|CreateWidget "/Game/LockPicking/W_Lock.W_Lock_C"))
        (bind _output_get_2 (Variables|Default|SetLockWidget _returnvalue)))
      (UserInterface|Viewport|AddtoViewport _output_get_2 0)
      (bind _output_get_3 (Variables|Default|SetPinRotation 0.0))
      (Class|Widget|SetRenderAngle (Variables|/Game/LockPicking/W_Lock.W_Lock_C|GetPin _output_get_2) _output_get_3)
      (bind _output_get_4 (Variables|Default|SetLockRotation 0.0))
      (Class|Widget|SetRenderAngle (Variables|/Game/LockPicking/W_Lock.W_Lock_C|GetLock _output_get_2) _output_get_4)
      (Variables|Default|SetbIsActive true)
      (else
        (Development|PrintString "Open Sesame!")))
    (else
      (Development|PrintString "No Picks!"))))

(event EventBeginPlay
  (Variables|Default|SetUnlockRotation (Math|Random|RandomFloatinRange -9e+01 9e+01))
  (bind _returnvalue (Utilities|GetDataTableRow "/Game/LockPicking/DT_LockDifficulty.DT_LockDifficulty" (Utilities|String|StringToName (Utilities|String|EnumtoString (Variables|Default|GetDifficulty))))
    (:then
      (Variables|Default|SetUnlockTolerance (.unlocktolerance _returnvalue))
      (Variables|Default|SetRotateTolerance (.rotatetolerance _returnvalue)))))

(fn ConstructionScript)