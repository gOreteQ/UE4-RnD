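; BP_ConnectionActor marks a connection point between rooms and places the door there.
; When active, PlaceDoor checks the first other connection actor overlapping its Sphere to determine whether it is connected.
; If that neighbor already placed a door, it deactivates, avoiding a duplicate.
; Otherwise it spawns a BP_RoomConnectionDoor at its transform, which can open only if connected, so unmatched connections get non-opening doors.
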(fn `PlaceDoor`
  (bind _item (`KismetArrayLibrary.Array_Get` (`PrimitiveComponent.GetOverlappingActors` (`self.Sphere`) "BP_ConnectionActor_C")))
  (if (`self.bActive`)
    (if (`KismetSystemLibrary.IsValid` _item)
      (set `self.bConnected` true)
      (if (`/Game/RGW/BP_ConnectionActor.bDoorPlaced` (cast `/Game/RGW/BP_ConnectionActor` _item :!pure true))
        (set `self.bActive` false)
        (else
          (bind _returnvalue (`|SpawnActorFromClass` "/Game/RGW/BP_RoomConnectionDoor.BP_RoomConnectionDoor_C" (`self.GetTransform`) "Undefined" "OverrideRootScale" :!label _label))
          (set `self.bDoorPlaced` true)
          (set `/Game/RGW/BP_RoomConnectionDoor.CanOpen?` (`self.bConnected`) _returnvalue)))
      (else
        (set `self.bConnected` false)
        (goto _label)))))

(fn `UserConstructionScript`)